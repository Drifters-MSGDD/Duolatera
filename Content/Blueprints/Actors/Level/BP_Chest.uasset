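; BP_Chest is a level chest that opens when activated and presents items on rising elevators.
; Activate runs a timeline that slides the lid aside and slightly up, then after a short delay raises the holster and fires the ChestOpened dispatcher.
; A separate SecondChestItemRaise event lifts the pistol elevator.
; Timelines lerp world locations from stored starts, though BeginPlay caches only the lid and holster positions, not the pistol's.
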(event `self.ReceiveBeginPlay`
  (set `self.InitialL_glass` (`SceneComponent.K2_GetComponentLocation` (`self.Chest_Top`)))
  (set `self.HolsterEla` (`SceneComponent.K2_GetComponentLocation` (`self.HolsterElavator`))))

(event `self.Activate`
  (`self.OpenChestAndFirstItem`))

(event `OpenChestAndFirstItem`
  (bind _initiall_glass (`self.InitialL_glass`))
  (bind _holsterela (`self.HolsterEla`))
  (bind (_direction _timeline) (`Timeline|TimeLine`)
    (:`Update`
      (`SceneComponent.K2_SetWorldLocation` (`self.Chest_Top`) (`KismetMathLibrary.VLerp` _initiall_glass (+ _initiall_glass (`KismetMathLibrary.MakeVector` (+ 90.0 0.0) 0.0 (+ 5.0 0.0))) _timeline) false false))
    (:`Finished`
      (`KismetSystemLibrary.Delay` 0.5)
      (bind (_direction_2 _timeline_2) (`Timeline|Timeline_1` :!via `PlayFromStart`)
        (:`Update`
          (`SceneComponent.K2_SetWorldLocation` (`self.HolsterElavator`) (`KismetMathLibrary.VLerp` _holsterela (+ _holsterela (0.0 0.0 40.0)) _timeline_2) false false))
        (:`Finished`
          (`self.ChestOpened`))))))

(event `SecondChestItemRaise`
  (bind _pistolela (`self.PistolEla`))
  (bind (_direction _timeline) (`Timeline|Timeline_0`)
    (:`Update`
      (`SceneComponent.K2_SetWorldLocation` (`self.PistolElavaor`) (`KismetMathLibrary.VLerp` _pistolela (+ _pistolela (0.0 0.0 40.0)) _timeline) false false))))

(fn `UserConstructionScript`)