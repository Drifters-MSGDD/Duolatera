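; BP_RingSensor is a capsule trigger that VR pawns switch on by reaching into it, driving its parent's interact begin and end calls.
; Entering and leaving play haptics on the motion controller found two attach levels above the overlapping component.
; Only the authority changes the activated state, switching on at first overlap.
; When no VR pawn remains, it switches off after a die-off delay, without rechecking overlaps.
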(event `self.Capsule.OnComponentBeginOverlap`
  (params (OverlappedComponent :type "PrimitiveComponent Object Reference") (OtherActor :type "Actor Object Reference") (OtherComp :type "PrimitiveComponent Object Reference") (OtherBodyIndex :type Integer) (bFromSweep :type Boolean) (SweepResult :type "HitResult Structure (by ref)"))
  (cast `/Game/Blueprints/Actors/VRPawn` OtherActor)
  (`|ExecutionSequence`
    (:`then_0`
      (bind _asmotion_controller_component (cast `MotionControllerComponent` (`SceneComponent.GetAttachParent` (`SceneComponent.GetAttachParent` OtherComp))))
      (`/Game/Blueprints/BlueprintFunctionLibrary.TriggerPlaysHapticEffect` _asmotion_controller_component (`self.hapticEffectEnter`)))
    (:`then_1`
      (`/Engine/EditorBlueprintResources/ActorMacros.Switch Has Authority`
        (:`Authority`
          (if (not (`self.bActivated`))
            (`self.Activate`)))))))

(event `self.Capsule.OnComponentEndOverlap`
  (params (OverlappedComponent :type "PrimitiveComponent Object Reference") (OtherActor :type "Actor Object Reference") (OtherComp :type "PrimitiveComponent Object Reference") (OtherBodyIndex :type Integer))
  (cast `/Game/Blueprints/Actors/VRPawn` OtherActor)
  (`|ExecutionSequence`
    (:`then_0`
      (bind _asmotion_controller_component (cast `MotionControllerComponent` (`SceneComponent.GetAttachParent` (`SceneComponent.GetAttachParent` OtherComp))))
      (`/Game/Blueprints/BlueprintFunctionLibrary.TriggerPlaysHapticEffect` _asmotion_controller_component (`self.hapticEffectExit`)))
    (:`then_1`
      (`/Engine/EditorBlueprintResources/ActorMacros.Switch Has Authority`
        (:`Authority`
          (if (and (`self.bActivated`) (== (`KismetArrayLibrary.Array_Length` (`PrimitiveComponent.GetOverlappingActors` (`self.Capsule`) "/Game/Blueprints/Actors/VRPawn.VRPawn_C")) 0))
            (`self.DelayInactivate`)))))))

(event `Activate`
  (set `self.bActivated` true)
  ;[0.2292 0.2292 0.2292] This calls the parent base implementation
  (`self.BeginInteract` null))

(event `DelayInactivate`
  (`KismetSystemLibrary.Delay` (`self.dieOffDelay`))
  (set `self.bActivated` false)
  ;[0.2292 0.2292 0.2292] This calls the parent base implementation
  (`self.EndInteract` null))

(fn `OnRep_bActivated`)

(fn `UserConstructionScript`)