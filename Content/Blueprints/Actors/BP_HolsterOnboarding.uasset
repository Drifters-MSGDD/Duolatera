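; VR onboarding actor: a grabbable holster that the player brings to their body to equip.
; BeginPlay hides the pawn's holster mesh and line-traces for floor height; within HolsterRadius of that mesh, the actor destroys itself and reveals it.
; If released below a floor-based height threshold, it pauses Tick and physics while a timeline lerps and slerps it back to its start transform, stopping if grabbed.
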(event `self.ReceiveBeginPlay`
  (bind (_raycaststartlocation_x _raycaststartlocation_y _raycaststartlocation_z) (`KismetMathLibrary.BreakVector` (`self.RayCastStartLocation`)))
  (bind _returnvalue (`GameplayStatics.GetActorOfClass` "/Game/Blueprints/Actors/VRPawn.VRPawn_C"))
  (set `self.VRPawn` _returnvalue)
  (bind _outhit (`KismetSystemLibrary.LineTraceSingle` :`Start` (`KismetMathLibrary.MakeVector` _raycaststartlocation_x _raycaststartlocation_y _raycaststartlocation_z) :`End` (`KismetMathLibrary.MakeVector` 0.0 0.0 (* _raycaststartlocation_z -1000.0)) :`TraceChannel` "TraceTypeQuery1" :`DrawDebugType` "ForDuration" :`DrawTime` 30.0))
  (bind (_returnvalue_x _returnvalue_y _returnvalue_z) (`KismetMathLibrary.BreakVector` (`self.K2_GetActorLocation` (`.HitActor` (`GameplayStatics.BreakHitResult` _outhit)))))
  (bind _output_get (set `self.FloorHeight` _returnvalue_z))
  (`KismetSystemLibrary.PrintString` (`KismetStringLibrary.Conv_DoubleToString` _output_get) true true (struct :`R` 1.0 :`G` 0.023719 :`B` 0.84045 :`A` 1.0) 40.0)
  (`self.SetActorTickEnabled` true)
  (set `self.StartLocation` (`SceneComponent.K2_GetComponentLocation` (`self.Holster`)))
  (set `self.StartRotation` (`SceneComponent.K2_GetComponentRotation` (`self.Holster`)))
  (`SceneComponent.SetVisibility` (`/Game/Blueprints/Actors/VRPawn.HolsterStaticMesh` (`self.VRPawn`)) false false))

(event `self.ReceiveTick`
  (params (DeltaSeconds :type "Float (single-precision)"))
  (bind (_returnvalue_x _returnvalue_y _returnvalue_z) (`KismetMathLibrary.BreakVector` (`SceneComponent.K2_GetComponentLocation` (`self.Holster`))))
  (bind (_returnvalue_x_2 _returnvalue_y_2 _returnvalue_z_2) (`KismetMathLibrary.BreakVector` (`SceneComponent.K2_GetComponentScale` (`self.Holster`))))
  (`/Engine/EditorBlueprintResources/StandardMacros.IsValid` (`self.VRPawn`)
    (:`Is Valid`
      (`|ExecutionSequence`
        (:`then_0`
          (if (< _returnvalue_z (+ (/ (`KismetMathLibrary.Abs` (`self.FloorHeight`)) 2.0) (/ (* _returnvalue_z_2 50.0) 2.0)))
            (if (not (`/Game/Blueprints/Components/GrabComponent.bIsHeld` (`self.GrabComponent`)))
              (`self.SetActorTickEnabled` false)
              (set `self.CurrentHolsterLocation` (`SceneComponent.K2_GetComponentLocation` (`self.Holster`)))
              (set `self.CurrentHolsterRotation` (`SceneComponent.K2_GetComponentRotation` (`self.Holster`)))
              (`self.TimelineSnap`))))
        (:`then_1`
          (if (<= (`KismetMathLibrary.VSize` (- (`SceneComponent.K2_GetComponentLocation` (`/Game/Blueprints/Actors/VRPawn.HolsterStaticMesh` (`self.VRPawn`))) (`SceneComponent.K2_GetComponentLocation` (`self.GrabComponent`)))) (`self.HolsterRadius`))
            (`/Engine/EditorBlueprintResources/StandardMacros.IsValid` (`self.Holster`)
              (:`Is Valid`
                (`self.SetActorTickEnabled` false)
                (`self.K2_DestroyActor`)
                (`SceneComponent.SetVisibility` (`/Game/Blueprints/Actors/VRPawn.HolsterStaticMesh` (`self.VRPawn`)) true false)))))))
    (:`Is Not Valid`
      (`KismetSystemLibrary.PrintString` "Not Valid" true true (struct :`R` 0.33953 :`G` 1.0 :`A` 1.0) 10.0))))

(event `TimelineSnap`
  (bind _holster (`self.Holster`))
  (`/Game/Blueprints/Components/GrabComponent.SetPrimitiveCompPhysics` (`self.GrabComponent`) false)
  (bind (_direction _snap) (`Timeline|Snap Holster to platform` :!via `PlayFromStart` :!label _label)
    (:`Update`
      (`|ExecutionSequence`
        (:`then_0`
          (bind _isheld (`/Game/Blueprints/Components/GrabComponent.CheckIfHeld` (`self.GrabComponent`)))
          (if _isheld
            (`KismetSystemLibrary.PrintString` "stopped" true true (struct :`G` 0.66 :`B` 1.0 :`A` 1.0) 10.0)
            (goto _label :!via `Stop`)))
        (:`then_1`
          (`SceneComponent.K2_SetWorldLocation` _holster (`KismetMathLibrary.VLerp` (`self.CurrentHolsterLocation`) (`self.StartLocation`) _snap) false false))
        (:`then_2`
          (`SceneComponent.K2_SetWorldRotation` _holster (`KismetMathLibrary.Quat_Rotator` (`KismetMathLibrary.Quat_Slerp` (`KismetMathLibrary.Conv_RotatorToQuaternion` (`self.CurrentHolsterRotation`)) (`KismetMathLibrary.Conv_RotatorToQuaternion` (`self.StartRotation`)) _snap)) false false))
        (:`then_3`
          (`KismetSystemLibrary.PrintString` (`KismetStringLibrary.Conv_DoubleToString` _snap)))))
    (:`Finished`
      (`self.SetActorTickEnabled` true)
      (`/Game/Blueprints/Components/GrabComponent.SetPrimitiveCompPhysics` (`self.GrabComponent`) true))))

(fn `UserConstructionScript`)