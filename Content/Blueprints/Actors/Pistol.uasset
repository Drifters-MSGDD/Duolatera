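; Replicated VR laser pistol that binds to its player by PlayerID, takes that player's color and returns to their holster when dropped, snapping if near or sweeping back after a cooldown.
; While firing, Tick runs a portal-aware trace that feeds the replicated Niagara beam points, and the authority notifies hit actors.
; RepNotifies drive beam, audio and tick state; overlapping an UnderworldRegion disables firing with a fizzle.
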(event `InitilizePistol`
  (params (playerID :type Integer))
  ;[1 1 1] Holster Stuff
  (set `self.PlayerID` playerID))

(event `BindOnDroppedEvent`
  ;[1 1 1] Holster Stuff
  (add `/Game/Blueprints/Components/GrabComponent.OnDropped` (`self.GrabComponentSnap`) (delegate `OnLaserToolDropped`))
  (`self.OnLaserToolDropped`))

(event `OnLaserToolDropped`
  (bind _skeletalmeshgun (`self.SkeletalMeshGun`))
  ;[1 1 1] Holster Stuff
  (`/Engine/EditorBlueprintResources/StandardMacros.IsValid` (`self.playerReference`)
    (:`Is Valid`
      (if (<= (`KismetMathLibrary.VSize` (- (`SceneComponent.K2_GetComponentLocation` (`/Game/Blueprints/Actors/VRPawn.HolsterStaticMesh` (`self.playerReference`))) (`SceneComponent.K2_GetComponentLocation` (`self.GrabComponentSnap`)))) (`self.snapHolsterRadius`))
        (`SceneComponent.K2_AttachToComponent` (`self.SkeletalMeshGun`) (`/Game/Blueprints/Actors/VRPawn.HolsterStaticMesh` (`self.playerReference`)) "None" "KeepWorld" "KeepWorld" "KeepWorld" false :!label _label)
        (else
          (`Timeline|AutoSnapCooldown` :!via `PlayFromStart`
            (:`Finished`
              (bind _isheld (`/Game/Blueprints/Components/GrabComponent.CheckIfHeld` (`self.GrabComponentSnap`)))
              (if (not _isheld)
                (`/Game/Blueprints/Components/GrabComponent.SetPrimitiveCompPhysics` (`self.GrabComponentSnap`) false)
                (`|ExecutionSequence`
                  (:`then_0`
                    ;;[1 1 1] set location & rotation for lerp
                    (set `self.tempWorldLocation` (`SceneComponent.K2_GetComponentLocation` (`self.SkeletalMeshGun`))))
                  (:`then_1`
                    (set `self.tempWorldRotation` (`SceneComponent.K2_GetComponentRotation` (`self.SkeletalMeshGun`))))
                  (:`then_2`
                    (bind (_direction _sweep) (`Timeline|SweepToHolster` :!via `PlayFromStart` :!label _label_2)
                      (:`Update`
                        (`|ExecutionSequence`
                          (:`then_0`
                            (bind _isheld_2 (`/Game/Blueprints/Components/GrabComponent.CheckIfHeld` (`self.GrabComponentSnap`)))
                            (if _isheld_2
                              (goto _label_2 :!via `Stop`)))
                          (:`then_1`
                            (`SceneComponent.K2_SetWorldLocation` _skeletalmeshgun (`KismetMathLibrary.VLerp` (`self.tempWorldLocation`) (`SceneComponent.K2_GetComponentLocation` (`/Game/Blueprints/Actors/VRPawn.HolsterStaticMesh` (`self.playerReference`))) _sweep) false true))
                          (:`then_2`
                            (`SceneComponent.K2_SetWorldRotation` _skeletalmeshgun (`KismetMathLibrary.Quat_Rotator` (`KismetMathLibrary.Quat_Slerp` (`KismetMathLibrary.Conv_RotatorToQuaternion` (`self.tempWorldRotation`)) (`KismetMathLibrary.Conv_RotatorToQuaternion` (`SceneComponent.K2_GetComponentRotation` (`/Game/Blueprints/Actors/VRPawn.HolsterStaticMesh` (`self.playerReference`)))) _sweep)) false true))))
                      (:`Finished`
                        (goto _label)))))))))))
    (:`Is Not Valid`
      (`KismetSystemLibrary.PrintString` "Error: This pistol could't find its lover" true true (struct :`G` 0.66 :`B` 1.0 :`A` 1.0) 302.0))))

(event `self.GrabComponentSnap.OnGrabbed`
  (`SceneComponent.SetVisibility` (`self.NS_LaserBeam`) false false :!label _label_3)
  (`PlayerController.StopHapticEffect` (`GameplayStatics.GetPlayerController` 0) (`/Game/Blueprints/Components/GrabComponent.GetHeldByHand` (`self.GrabComponentSnap`)))
  (`AudioComponent.Stop` (`self.Cue_LaserFireLoop`))
  (`self.server set firing` false))

(event `self.SkeletalMeshGun.OnComponentBeginOverlap`
  (params (OverlappedComponent :type "PrimitiveComponent Object Reference") (OtherActor :type "Actor Object Reference") (OtherComp :type "PrimitiveComponent Object Reference") (OtherBodyIndex :type Integer) (bFromSweep :type Boolean) (SweepResult :type "HitResult Structure (by ref)"))
  ;[1 0.4734 0.2717] Set laser fireable or not whether it enters or leaves the underworld
  (if (`ActorComponent.ComponentHasTag` OtherComp "UnderworldRegion")
    (set `self.fireable` false)))

(event `self.EndInteract`
  (params (heldController :type "MotionControllerComponent Object Reference"))
  (goto _label_3))

(event `self.GrabComponentSnap.OnDropped`
  (goto _label_3))

(event `self.SkeletalMeshGun.OnComponentEndOverlap`
  (params (OverlappedComponent :type "PrimitiveComponent Object Reference") (OtherActor :type "Actor Object Reference") (OtherComp :type "PrimitiveComponent Object Reference") (OtherBodyIndex :type Integer))
  ;[1 0.4734 0.2717] Set laser fireable or not whether it enters or leaves the underworld
  (if (`ActorComponent.ComponentHasTag` OtherComp "UnderworldRegion")
    (set `self.fireable` true)))

(event `server set firing`
  (params (enabled :type Boolean))
  (set `self.firing` enabled))

(event `self.BeginInteract`
  (params (heldController :type "MotionControllerComponent Object Reference"))
  ;[0.7838 1 0.4879] Begin firing the laser if it's fireable. If not, just play the fizzle sound.
  (`/Engine/EditorBlueprintResources/StandardMacros.DoOnce` false :!label _label_4
    (:`Completed`
      (`|ExecutionSequence`
        (:`then_0`
          (`KismetSystemLibrary.Delay` 0.2)
          (goto _label_4 :!via `Reset`))
        (:`then_1`
          (if (`self.fireable`)
            (`PlayerController.PlayHapticEffect` (`GameplayStatics.GetPlayerController` 0) "/Game/Haptics/PistolFireHapticEffect.PistolFireHapticEffect" (`/Game/Blueprints/Components/GrabComponent.GetHeldByHand` (`self.GrabComponentSnap`)) 0.5 true)
            (`SceneComponent.SetVisibility` (`self.NS_LaserBeam`) true false)
            (`AudioComponent.Play` (`self.Cue_LaserFireStart`) 0.0)
            (`AudioComponent.Play` (`self.Cue_LaserFireLoop`) 0.0)
            (`self.SetActorTickEnabled` true)
            (`self.server set firing` true)
            (else
              (`PlayerController.PlayHapticEffect` (`GameplayStatics.GetPlayerController` 0) "/Game/Haptics/TriggerHapticEffect.TriggerHapticEffect" (`/Game/Blueprints/Components/GrabComponent.GetHeldByHand` (`self.GrabComponentSnap`)) 3.0 false)
              (`AudioComponent.Play` (`self.Cue_LaserFizzle`) 0.0))))))))

(event `self.ReceiveTick`
  (params (DeltaSeconds :type "Float (single-precision)"))
  (bind _muzzlelocation (`self.MuzzleLocation`))
  (bind (_outhit _outportalhit _tracedthroughportal _returnvalue) (`ExtraBlueprintFunctionLibrary.PortalLineTrace` :`Start` (`SceneComponent.K2_GetComponentLocation` _muzzlelocation) :`Direction` (`SceneComponent.GetForwardVector` _muzzlelocation) :`Distance` (`self.laserRange`) :`TraceChannel` "TraceTypeQuery1" :`DrawTime` 1.0))
  (if _returnvalue
    (bind (_bblockinghit _binitialoverlap _time _distance _location _impactpoint _normal _impactnormal _physmat _hitactor _hitcomponent _hitbonename _bonename _hititem _elementindex _faceindex _tracestart _traceend) (`GameplayStatics.BreakHitResult` _outhit))
    (set `self.impactPt` _impactpoint)
    (bind (_bblockinghit_2 _binitialoverlap_2 _time_2 _distance_2 _location_2 _impactpoint_2 _normal_2 _impactnormal_2 _physmat_2 _hitactor_2 _hitcomponent_2 _hitbonename_2 _bonename_2 _hititem_2 _elementindex_2 _faceindex_2 _tracestart_2) (`GameplayStatics.BreakHitResult` _outportalhit))
    (set `self.laserPtsArray` (select `bool` _tracedthroughportal :`false` (`|MakeArray` _tracestart _impactpoint) :`true` (`|MakeArray` _tracestart_2 _impactpoint_2 _tracestart _impactpoint)))
    (`/Engine/EditorBlueprintResources/ActorMacros.Switch Has Authority`
      (:`Authority`
        (message `Taggable.OnTagged` (`.HitActor` (`GameplayStatics.BreakHitResult` _outhit)) _outhit)))
    (else
      (set `self.impactPt` (99999.0 99999.0 99999.0))
      (set `self.laserPtsArray` (select `bool` _tracedthroughportal :`false` (`|MakeArray` _tracestart _traceend) :`true` (`|MakeArray` _tracestart_2 _impactpoint_2 _tracestart _traceend))))))

(fn `OnRep_fireable`
  (bind _grabcomponentsnap (`self.GrabComponentSnap`))
  (if (`/Game/Blueprints/Components/GrabComponent.bIsHeld` _grabcomponentsnap)
    (`PlayerController.PlayHapticEffect` (`GameplayStatics.GetPlayerController` 0) "/Game/Haptics/TriggerHapticEffect.TriggerHapticEffect" (`/Game/Blueprints/Components/GrabComponent.GetHeldByHand` _grabcomponentsnap) 3.0 false))
  (if (not (`self.fireable`))
    (`self.SetActorTickEnabled` false)
    (`AudioComponent.Stop` (`self.Cue_LaserFireLoop`))
    (`AudioComponent.Play` (`self.Cue_LaserFizzle`) 0.0)
    (`SceneComponent.SetVisibility` (`self.NS_LaserBeam`) false false)))

(fn `OnRep_firing`
  (bind _firing (`self.firing`))
  (bind _cue_laserfireloop (`self.Cue_LaserFireLoop`))
  (`self.SetActorTickEnabled` (and (`self.fireable`) _firing))
  (`SceneComponent.SetVisibility` (`self.NS_LaserBeam`) _firing false)
  (if _firing
    (if (not (`AudioComponent.IsPlaying` _cue_laserfireloop))
      (`AudioComponent.Play` (`self.Cue_LaserFireStart`) 0.0)
      (`AudioComponent.Play` _cue_laserfireloop 0.0))
    (else
      (`AudioComponent.Stop` _cue_laserfireloop))))

(fn `OnRep_GunMaterial`
  (`PrimitiveComponent.SetMaterial` (`self.SkeletalMeshGun`) 0 (`self.GunMaterial`)))

(fn `OnRep_impactPt`
  (`NiagaraComponent.SetVariablePosition` (`self.NS_LaserBeam`) "LaserEnd" (`self.impactPt`)))

(fn `OnRep_laserPtsArray`
  (`NiagaraDataInterfaceArrayFunctionLibrary.SetNiagaraArrayVector` (`self.NS_LaserBeam`) "LaserPoints" (`self.laserPtsArray`)))

(fn `OnRep_PlayerID`
  (bind _skeletalmeshgun (`self.SkeletalMeshGun`))
  (`|ExecutionSequence`
    (:`then_0`
      (bind _outactors (`GameplayStatics.GetAllActorsOfClass` "/Game/Blueprints/Actors/VRPawn.VRPawn_C"))
      (for _array_element _outactors
        (if (== (`/Game/Blueprints/Actors/VRPawn.PlayerID` _array_element) (`self.PlayerID`))
          (set `self.playerReference` _array_element)
          (break))))
    (:`then_1`
      (switch `int` (`self.PlayerID`)
        (:`Default`
          (`KismetSystemLibrary.PrintString` "Error from Pistol::InitializePistol, player ID is not 0 or 1, invliad ID" true true (struct :`R` 1.0 :`G` 0.013146 :`A` 1.0) 60.0))
        (:`0`
          (`PrimitiveComponent.SetMaterial` _skeletalmeshgun 0 "/Game/Assets/Materials/MaterialInstance/MI_Pistol_Blue.MI_Pistol_Blue"))
        (:`1`
          (`PrimitiveComponent.SetMaterial` _skeletalmeshgun 0 "/Game/Assets/Materials/MaterialInstance/MI_Pistol_Green.MI_Pistol_Green"))))
    (:`then_2`
      (`self.BindOnDroppedEvent`))
    (:`then_3`
      (`SceneComponent.SetWorldScale3D` (`self.SkeletalMeshGun`) (`KismetMathLibrary.Conv_DoubleToVector` 0.5)) ; When the client joins, it sees the host's gun with 1.0 scale, so we're setting the pistol's scale manually
    )))

(fn `UserConstructionScript`)