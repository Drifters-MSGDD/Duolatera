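; BP_Gate is a replicated iris-style gate that opens and closes through Activate/Deactivate, which set Opend.
; Its OnRep runs the animation, toggles gateway blocker collision and calls opened/closed dispatches.
; A reversible timeline slides radially arranged sectors outward and slerps them from construction-cached rotations, deriving directions from sector count and mesh axes.
; Open and close sounds start at offsets based on animation progress, so mid-motion reversals stay in sync.
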(event `OpenGate`
  (bind _door_open_cue (`self.Door Open Cue`))
  (bind _sm_gateframe (`self.SM_GateFrame`))
  (bind _gatesectors (`self.gateSectors`))
  (`AudioComponent.Stop` (`self.Door Close Cue`))
  (`AudioComponent.Play` _door_open_cue (`KismetMathLibrary.Lerp` 0.0 (* (`SoundBase.Duration` (`AudioComponent.Sound` _door_open_cue)) 0.8) (`self.animTime`)))
  (bind (_direction _tltrack) (`Timeline|GateAnimation` :!label _label)
    (:`Update`
      (bind _output_get (set `self.animTime` _tltrack))
      (for (_array_element _array_index) _gatesectors
        (bind _output (`|GetArrayItem` (`self.initialTransforms`) _array_index))
        (`SceneComponent.K2_SetRelativeLocationAndRotation` _array_element (`KismetMathLibrary.VLerp` (0.0 0.0 0.0) (+ (`KismetMathLibrary.Vector_Zero`) (* (`KismetMathLibrary.RotateAngleAxis` (`KismetMathLibrary.InverseTransformDirection` (`SceneComponent.K2_GetComponentToWorld` _array_element) (`SceneComponent.GetUpVector` _array_element)) (`KismetMathLibrary.Conv_IntToDouble` (* _array_index (`KismetMathLibrary.SafeDivide` -360.0 (`KismetMathLibrary.Conv_IntToDouble` (`KismetArrayLibrary.Array_Length` _gatesectors))))) (`KismetMathLibrary.InverseTransformDirection` (`SceneComponent.K2_GetComponentToWorld` _sm_gateframe) (`SceneComponent.GetForwardVector` _sm_gateframe))) (`self.sectorMoveDistance`))) _output_get) (`KismetMathLibrary.Quat_Rotator` (`KismetMathLibrary.Quat_Slerp` (`KismetMathLibrary.Conv_RotatorToQuaternion` _output) (`KismetMathLibrary.Conv_RotatorToQuaternion` (`KismetMathLibrary.ComposeRotators` _output (`KismetMathLibrary.MakeRotator` (`self.sectorRotateAngle`)))) _output_get)) false false)))))

(event `CloseGate`
  (bind _door_close_cue (`self.Door Close Cue`))
  (`AudioComponent.Stop` (`self.Door Open Cue`))
  (`AudioComponent.Play` _door_close_cue (`KismetMathLibrary.Lerp` (* (`SoundBase.Duration` (`AudioComponent.Sound` _door_close_cue)) 0.55) 0.0 (`self.animTime`)))
  (goto _label :!via `Reverse`))

(event `DisableGatewayCollision`
  (`PrimitiveComponent.SetCollisionEnabled` (`self.GatewayBlock`) "NoCollision"))

(event `EnableGatewayCollision`
  (`PrimitiveComponent.SetCollisionEnabled` (`self.GatewayBlock`) "QueryAndProbe"))

(event `self.Activate`
  (set `self.bOpend` true))

(event `self.Deactivate`
  (set `self.bOpend` false))

(fn `OnRep_bOpend`
  (if (`self.bOpend`)
    (`self.OpenGate`)
    (`self.DisableGatewayCollision`)
    (`self.OnOpenedDispatch`)
    (else
      (`self.CloseGate`)
      (`self.EnableGatewayCollision`)
      (`self.OnClosedDispatch`))))

(fn `UserConstructionScript`
  (bind _gatesectors (`self.gateSectors`))
  (`|ExecutionSequence`
    (:`then_0`
      (`KismetArrayLibrary.Array_Add` _gatesectors (`self.SM_GateSector`))
      (`KismetArrayLibrary.Array_Add` _gatesectors (`self.SM_GateSector1`))
      (`KismetArrayLibrary.Array_Add` _gatesectors (`self.SM_GateSector2`))
      (`KismetArrayLibrary.Array_Add` _gatesectors (`self.SM_GateSector3`))
      (`KismetArrayLibrary.Array_Add` _gatesectors (`self.SM_GateSector4`))
      (`KismetArrayLibrary.Array_Add` _gatesectors (`self.SM_GateSector5`))
      (`KismetArrayLibrary.Array_Add` _gatesectors (`self.SM_GateSector6`))
      (`KismetArrayLibrary.Array_Add` _gatesectors (`self.SM_GateSector7`)))
    (:`then_1`
      (for _array_element (`self.gateSectors`)
        (`KismetArrayLibrary.Array_Add` (`self.initialTransforms`) (`SceneComponent.RelativeRotation` _array_element))))))