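; VR game state that owns the linked Over and Under portal pair, moved between PortalCanvases, and tracks whether the local player is in the Underworld.
; On BeginPlay it spawns both portals off-map plus a global post-process actor, then subscribes to every canvas's draw event.
; Draw events reset previous canvases, while traversal and draw events choose which portal renders.
; RefreshGameState parks the portals and rebinds canvases after sublevel loads.
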(event `self.ReceiveBeginPlay`
  (bind _overportal (`self.overPortal`))
  (bind _underportal (`self.underPortal`))
  (bind _portal_component (`/Game/Blueprints/Actors/BP_Portal.Portal Component` (`self.overPortal`)))
  (`|ExecutionSequence`
    (:`then_0`
      ;[0.3429 0.4167 0.4167] When the game starts, create the 2 portals. These will be moved between the active canvases in the game
      (bind _returnvalue (`|SpawnActorFromClass` "/Game/Blueprints/Actors/BP_Portal.BP_Portal_C" (`KismetMathLibrary.MakeTransform` (-99999.0 -99999.0 -99999.0)) "AlwaysSpawn" "MultiplyWithRoot" null null))
      (set `self.overPortal` _returnvalue)
      (bind _returnvalue_2 (`|SpawnActorFromClass` "/Game/Blueprints/Actors/BP_Portal.BP_Portal_C" (`KismetMathLibrary.MakeTransform` (-99999.0 -99999.0 -99999.0)) "AlwaysSpawn" "MultiplyWithRoot" null null))
      (bind _output_get (set `self.underPortal` _returnvalue_2))
      (bind _portal_component_2 (`/Game/Blueprints/Actors/BP_Portal.Portal Component` _output_get))
      (`PortalComponent.SetDestinationPortal` _portal_component_2 _portal_component)
      (`PortalComponent.SetDestinationPortal` _portal_component _portal_component_2)
      (`self.OnPortalsCreated` _overportal _underportal)
      (add `PortalComponent.OnPortalTraversed` (`/Game/Blueprints/Actors/BP_Portal.Portal Component` _overportal) (delegate `OnPortalTraversed_Event`))
      (add `PortalComponent.OnPortalTraversed` (`/Game/Blueprints/Actors/BP_Portal.Portal Component` _underportal) (delegate `OnPortalTraversed_Event`)))
    (:`then_1`
      ;[0.6927 0.6019 0.31] Grab ref to postprocess actor. If none was found, make one here. This will be used immediately by the Portal Components spawned above.
      (bind _returnvalue_3 (`|SpawnActorFromClass` "/Script/Duolatera.GlobalPostProcess" (`KismetMathLibrary.MakeTransform` (0.0 0.0 0.0)) "Undefined" "MultiplyWithRoot" null null))
      (set `self.globalPP` _returnvalue_3))
    (:`then_2`
      ;[0.4635 0.4635 0.4635] We need to listen for the Portal Drawn events of all portal canvases in the game. Therefore this block needs to run every time a new sublevel is loaded, so the ListenForPortalCanvasDrawEvents event is called from BP_LevelLoader to handle this.
      (bind _outactors (`GameplayStatics.GetAllActorsOfClass` "/Script/Duolatera.PortalCanvas" :!label _label))
      (for _array_element _outactors
        (add `PortalCanvas.OnPortalDrawn` _array_element (delegate `OnPortalDrawn_Event`))))))

(event `OnPortalTraversed_Event`
  (params (object :type "Actor Object Reference") (fromPortal :type "PortalComponent Object Reference") (toPortal :type "PortalComponent Object Reference"))
  ;[0.724 0.2925 0.2709] This switches the actively rendered portal whenever the local player moves through one. It then checks if they are now in the Underworld, and sets the PostProcess attributes accordingly.
  (bind _asvrpawn (cast `/Game/Blueprints/Actors/VRPawn` object))
  (if (`Pawn.IsLocallyControlled` _asvrpawn)
    (`PortalComponent.RenderThisPortal` toPortal)
    (bind _asportal_canvas (cast `PortalCanvas` (`self.GetAttachParentActor` (`ActorComponent.GetOwner` toPortal))))
    (set `self.Player In Underworld` (`PortalCanvas.isUnderworldCanvas` _asportal_canvas))))

(event `RefreshGameState`
  (`self.K2_SetActorLocation` (`self.overPortal`) (-99999.0 -99999.0 -99999.0) false false)
  (`self.K2_SetActorLocation` (`self.underPortal`) (-99999.0 -99999.0 -99999.0) false false)
  (goto _label))

(event `OnPortalDrawn_Event`
  (params (newCanvas :type "PortalCanvas Object Reference"))
  (bind _activecanvas (`self.activeCanvas`))
  (bind _destinationcanvas (`/Game/Blueprints/Actors/BP_PortalCanvas.DestinationCanvas` _activecanvas))
  ;[0.7708 0.331 0.4879] This event handles resetting the old portal canvases back to their original state after a new set of portal canvases are drawn on. If this doesn't happen, the old portal canvases will be empty with nothing to draw on later!
  (if (not (== newCanvas _activecanvas))
    (`/Engine/EditorBlueprintResources/StandardMacros.IsValid` _activecanvas
      (:`Is Valid`
        (`PortalCanvas.ResetCanvasPlanes` _activecanvas)
        (if (not (== _destinationcanvas (`/Game/Blueprints/Actors/BP_PortalCanvas.DestinationCanvas` newCanvas)))
          (`PortalCanvas.ResetCanvasPlanes` _destinationcanvas)
          (set `self.activeCanvas` newCanvas :!label _label_2)
          (`PortalComponent.RenderThisPortal` (select `bool` (`self.Player In Underworld`) :`false` (`/Game/Blueprints/Actors/BP_Portal.Portal Component` (`self.overPortal`)) :`true` (`/Game/Blueprints/Actors/BP_Portal.Portal Component` (`self.underPortal`))))))
      (:`Is Not Valid`
        (goto _label_2)))))

(fn `UserConstructionScript`)